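; Enemy deck actor for a card game that builds, displays and deals the enemy player's cards.
; On BeginPlay it spawns mana, creature and landscape cards into PlayerDeck, shuffles them and links to the EnemyPlayerCharacter.
; It then stacks the cards on the board, deals five into the player's hand by card type and displays that hand.
; DrawCard moves the last deck card to the hand and reorders it.
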(event `DrawCard`
  (bind _playerdeck (`self.PlayerDeck`))
  (bind _myplayer (`self.myPlayer`))
  (bind _returnvalue (- (`KismetArrayLibrary.Array_Length` _playerdeck) 1))
  ;[1 1 1] Robar carta del mazo
  (`KismetArrayLibrary.Array_Add` (`/Game/WoN/Blueprints/Player/EnemyPlayerCharacter.PlayerHand` _myplayer) (`|GetArrayItem` _playerdeck _returnvalue))
  (`KismetArrayLibrary.Array_Remove` _playerdeck _returnvalue)
  (`/Game/WoN/Blueprints/Player/EnemyPlayerCharacter.OrderMyHand` _myplayer))

(event `Create first hand`
  (bind _playerhand (`/Game/WoN/Blueprints/Player/EnemyPlayerCharacter.PlayerHand` (`self.myPlayer`)))
  ;[1 1 1] Obtener mano inicial
  (for _index (range 5)
    (bind _returnvalue (- (`self.tamDeck`) _index))
    (bind _output (`|GetArrayItem` (`self.PlayerDeck`) _returnvalue))
    (bind _ascard (cast `/Game/WoN/Blueprints/Cards/Card` _output)
      (:`then`
        (`KismetSystemLibrary.PrintString` "CARTA CRIATURA")
        (`KismetArrayLibrary.Array_Add` _playerhand _ascard))
      (:`CastFailed`
        (bind _asmana_card (cast `/Game/WoN/Blueprints/Cards/ManaCard` _output)
          (:`then`
            (`KismetSystemLibrary.PrintString` "Carta mana")
            (`KismetArrayLibrary.Array_Add` _playerhand _asmana_card))
          (:`CastFailed`
            (bind _aslandscape_card (cast `/Game/WoN/Blueprints/Cards/LandscapeCard` _output))
            (`KismetSystemLibrary.PrintString` "CARTA ESCENARIO")
            (`KismetArrayLibrary.Array_Add` _playerhand _aslandscape_card)))))
    (`KismetArrayLibrary.Array_Remove` (`self.PlayerDeck`) _returnvalue)))

(event `DisplayDeckCards`
  ;[1 1 1] Display deck in the board
  (for _array_element (`self.PlayerDeck`)
    (`self.K2_SetActorLocation` _array_element (`self.deckPosition`) false false)
    (`self.K2_SetActorRotation` _array_element (struct :`Yaw` -90.0 :`Roll` 90.0) false)
    (set `self.deckPosition` (+ (`self.deckPosition`) (0.0 0.0 6.0)))))

(event `self.ReceiveBeginPlay`
  ;[1 1 1] Inicializar mazo
  (`self.AddManaToDeck` 13)
  (`self.AddCreatureToDeck` 8)
  (`self.AddLandscapeToDeck` 1)
  (`KismetSystemLibrary.PrintString` (`KismetStringLibrary.Concat_StrStr` "CARTAS DEL MAZO: " (`KismetStringLibrary.Conv_IntToString` (`self.tamDeck`))) true true (struct :`R` 1.0 :`G` 0.631249 :`A` 1.0) 5.0)
  (`KismetArrayLibrary.Array_Shuffle` (`self.PlayerDeck`))
  ;;[1 1 1] Asociamos mazo con jugador
  (bind _outactors (`GameplayStatics.GetAllActorsOfClass` "/Game/WoN/Blueprints/Player/EnemyPlayerCharacter.EnemyPlayerCharacter_C"))
  (for _array_element _outactors
    (set `self.myPlayer` _array_element)
    (`self.DisplayDeckCards`)
    (`self.Create first hand`)
    (`/Game/WoN/Blueprints/Player/EnemyPlayerCharacter.DisplayHand` (`self.myPlayer`))))

(event `AddManaToDeck`
  (params (numCards :type Integer :default 5))
  ;[1 1 1] Add mana cards to my Deck
  (for _ (range 1 (+ numCards 1))
    (bind _returnvalue (`|SpawnActorFromClass` "/Game/WoN/Blueprints/Cards/ManaCard.ManaCard_C" (`KismetMathLibrary.MakeTransform` (-451.0 647.0 63.0) (struct :`Yaw` -90.0 :`Roll` 90.0)) "Undefined" "OverrideRootScale" null (struct) null (0.0 0.0 0.0) null))
    (bind _output_get (set `self.myManaCard` _returnvalue))
    (`/Game/WoN/Blueprints/Cards/ManaCard.CreateManaCard` _output_get)
    (`KismetArrayLibrary.Array_Add` (`self.PlayerDeck`) (`self.myManaCard`))
    ;;[1 1 1] Añadir a array invididual
    (`/Engine/EditorBlueprintResources/StandardMacros.IncrementInt` (`self.tamDeck`))))

(event `AddLandscapeToDeck`
  (params (numLands :type Integer :default 2))
  ;[1 1 1] Add landscape cards to my Deck
  (for _ (range 1 (+ numLands 1))
    (bind _returnvalue (`|SpawnActorFromClass` "/Game/WoN/Blueprints/Cards/LandscapeCard.LandscapeCard_C" (`KismetMathLibrary.MakeTransform` (-451.0 861.0 63.0) (struct :`Yaw` -90.0 :`Roll` 90.0)) "Undefined" "OverrideRootScale" null (struct) null false 0 false null))
    (bind _output_get (set `self.myLandCard` _returnvalue))
    (`/Game/WoN/Blueprints/Cards/LandscapeCard.CreateLandscapeCard` _output_get (-451.0 861.0 63.0))
    (`KismetArrayLibrary.Array_Add` (`self.PlayerDeck`) (`self.myLandCard`))
    (`/Engine/EditorBlueprintResources/StandardMacros.IncrementInt` (`self.tamDeck`))))

(event `AddCreatureToDeck`
  (params (LastIndex :type Integer :default 5))
  ;[1 1 1] Add creature cards to my Deck
  (for _ (range 1 (+ LastIndex 1))
    (bind _returnvalue (`|SpawnActorFromClass` "/Game/WoN/Blueprints/Cards/Card.Card_C" (`KismetMathLibrary.MakeTransform` (-1000.0 0.0 0.0) (struct :`Yaw` -90.0 :`Roll` 90.0)) "Undefined" "OverrideRootScale" null (struct) null false 0 false null))
    (`self.K2_SetActorLocation` _returnvalue (`self.PositionVector`) false false)
    (bind _output_get (set `self.myCreatureCard` _returnvalue))
    (`/Game/WoN/Blueprints/Cards/Card.CreateCard` _output_get "NewEnumerator3" (`self.PositionVector`))
    (`KismetArrayLibrary.Array_Add` (`self.PlayerDeck`) (`self.myCreatureCard`))
    (`/Engine/EditorBlueprintResources/StandardMacros.IncrementInt` (`self.tamDeck`))))

(fn `UserConstructionScript`)