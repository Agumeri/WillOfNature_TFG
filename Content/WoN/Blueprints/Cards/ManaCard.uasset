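; Mana card actor for a card game, which becomes a random land on BeginPlay and adds mana to the pool when clicked.
; Setup picks a land name from an enum, sets the name text and type and image materials, moves to a start position and caches the player character.
; The first click calls the Tablero board's AddManaToPool, teleports the card to the mana position and removes it from the player's hand.
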(event `self.ReceiveActorOnClicked`
  (params (ButtonPressed :type "Key Structure"))
  ;[1 1 1] Mover mana al sitio del mana
  (bind _outactors (`GameplayStatics.GetAllActorsOfClass` "/Game/WoN/Blueprints/Tablero/Tablero.Tablero_C"))
  (for _array_element _outactors
    (if (not (`self.isAdded`))
      (`/Game/WoN/Blueprints/Tablero/Tablero.AddManaToPool` _array_element)
      (set `self.isAdded` true)
      (`self.K2_SetActorLocation` (`self.ManaPositionVector`))
      (set `self.ManaPositionVector` (+ (`self.ManaPositionVector`) (0.0 0.0 3.0)))
      (`/Game/WoN/Blueprints/Player/PuzzlePlayerCharacter.RemoveCardFromHand` (`self.Player`) self))))

(event `SetCardLocation`
  (params (myNewPosition :type "Vector Structure"))
  ;[1 1 1] Set card location (for reposition use only)
  (`self.K2_SetActorLocation` myNewPosition))

(event `CreateManaCard`
  ;[1 1 1] Create Mana Card
  (bind _output_get (set `self.CardValues` (make `/Game/WoN/Blueprints/Cards/card_structure` (`|GetEnumeratorNameAsString` (cast `/Game/WoN/Blueprints/Cards/Lists/LandName` (`KismetMathLibrary.Conv_IntToByte` (`KismetMathLibrary.RandomIntegerInRange` 0 (- (enumcount `/Game/WoN/Blueprints/Cards/Lists/LandName`) 1))))))))
  (`self.SetCard` (break `/Game/WoN/Blueprints/Cards/card_structure` _output_get)))

(event `SetCardMaterial`
  (bind (_cardvalues_name _cardvalues_type) (break `/Game/WoN/Blueprints/Cards/card_structure` (`self.CardValues`)))
  ;[1 1 1] Set Card Material (Different material due to Card Type)
  (switch `/Game/WoN/Blueprints/Cards/Lists/CardTypes` _cardvalues_type
    (:`NewEnumerator0`
      (set `self.Material` "/Game/Puzzle/Meshes/OrangeMaterial.OrangeMaterial"))
    (:`NewEnumerator1`
      (set `self.Material` "/Game/WoN/Assets/Materials/Land_Card.Land_Card"))
    (:`NewEnumerator2`
      (set `self.Material` "/Game/WoN/Assets/Materials/Spell_Card.Spell_Card"))
    (:`NewEnumerator3`
      (set `self.Material` "/Game/WoN/Assets/Materials/Criature_Card.Criature_Card"))
    (:`NewEnumerator4`
      (set `self.Material` "/Game/WoN/Assets/Materials/Object_Card.Object_Card")))
  (`PrimitiveComponent.SetMaterial` (`self.CardBody`) 0 (`self.Material`)))

(event `SetManaImage`
  (params (Image :type String))
  ;[1 1 1] Set Mana Image
  (switch `string` Image
    (:`Pradera`
      (`PrimitiveComponent.SetMaterial` (`self.CardImage`) 0 "/Game/WoN/Assets/Materials/Pradera.Pradera"))
    (:`Montaña`
      (`PrimitiveComponent.SetMaterial` (`self.CardImage`) 0 "/Game/WoN/Assets/Materials/Montaña.Montaña"))
    (:`Playa`
      (`PrimitiveComponent.SetMaterial` (`self.CardImage`) 0 "/Game/WoN/Assets/Materials/Playa.Playa"))
    (:`Ciudad`
      (`PrimitiveComponent.SetMaterial` (`self.CardImage`) 0 "/Game/WoN/Assets/Materials/Ciudad.Ciudad"))))

(event `SetCard`
  (params (`Card Values Name` :type String) (`Card Values Type` :type "/Game/WoN/Blueprints/Cards/Lists/CardTypes Enum" :default "NewEnumerator0") (`Card Values LP` :type Integer) (`Card Values AP` :type Integer))
  (bind _cardvalues_name (break `/Game/WoN/Blueprints/Cards/card_structure` (`self.CardValues`)))
  ;[1 1 1] Set card values
  (set `self.CardValues` (make `/Game/WoN/Blueprints/Cards/card_structure` `Card Values Name` `Card Values Type` false `Card Values LP` `Card Values AP`))
  (`TextRenderComponent.K2_SetText` (`self.CardName`) (`KismetTextLibrary.Conv_StringToText` _cardvalues_name))
  (`self.SetCardMaterial`)
  (`self.SetManaImage` _cardvalues_name))

(event `self.ReceiveBeginPlay`
  ;[1 1 1] Inicializar valores
  (`self.CreateManaCard`)
  (`self.K2_SetActorLocation` (`self.posInicial`))
  (bind _outactors (`GameplayStatics.GetAllActorsOfClass` "/Game/WoN/Blueprints/Player/PuzzlePlayerCharacter.PuzzlePlayerCharacter_C"))
  (for _array_element _outactors
    (set `self.Player` _array_element)))

(fn `UserConstructionScript`)