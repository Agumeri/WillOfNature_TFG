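; Card actor for a card game that displays name, attack, life, skill and mana cost on a 3D card.
; CreateCard handles only creatures, randomizing name, stats, skill and cost.
; SetCard refreshes the texts, type-based body material and name-matched artwork, and ModValues reuses it for stat changes.
; Clicking toggles a fixed enlarged view, offering the CastCreature widget if uncast, or returns the card to its initial position.
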(event `CreateCard`
  (params (Selection :type "/Game/WoN/Blueprints/Cards/Lists/CardTypes Enum" :default "NewEnumerator0") (posInicial :type "Vector Structure"))
  ;[1 1 1] Create card
  (set `self.posInicial` posInicial)
  (switch `/Game/WoN/Blueprints/Cards/Lists/CardTypes` Selection
    (:`NewEnumerator3`
      (`self.CreateCreatureCard` Selection))))

(event `SetCreatureImage`
  (params (A :type String))
  ;[1 1 1] Set Creature Image
  (switch `string` A
    (:`Lobo`
      (`PrimitiveComponent.SetMaterial` (`self.CardImage`) 0 "/Game/WoN/Assets/Materials/Perro.Perro"))
    (:`Salaryman`
      (`PrimitiveComponent.SetMaterial` (`self.CardImage`) 0 "/Game/WoN/Assets/Materials/Salaryman.Salaryman"))
    (:`Abuelita`
      (`PrimitiveComponent.SetMaterial` (`self.CardImage`) 0 "/Game/WoN/Assets/Materials/Abuelita.Abuelita"))
    (:`Patata`
      (`PrimitiveComponent.SetMaterial` (`self.CardImage`) 0 "/Game/WoN/Assets/Materials/Patata.Patata"))
    (:`F1 Ferrari`
      (`PrimitiveComponent.SetMaterial` (`self.CardImage`) 0 "/Game/WoN/Assets/Materials/Tronchamulas.Tronchamulas"))
    (:`Gato negro`
      (`PrimitiveComponent.SetMaterial` (`self.CardImage`) 0 "/Game/WoN/Assets/Materials/GatoNegro.GatoNegro"))
    (:`Asesino`
      (`PrimitiveComponent.SetMaterial` (`self.CardImage`) 0 "/Game/WoN/Assets/Materials/Asesino.Asesino"))
    (:`Barbol`
      (`PrimitiveComponent.SetMaterial` (`self.CardImage`) 0 "/Game/WoN/Assets/Materials/Barbol.Barbol"))
    (:`Golem`
      (`PrimitiveComponent.SetMaterial` (`self.CardImage`) 0 "/Game/WoN/Assets/Materials/Filemon.Filemon"))
    (:`Tortuga`
      (`PrimitiveComponent.SetMaterial` (`self.CardImage`) 0 "/Game/WoN/Assets/Materials/Tortuga.Tortuga"))
    (:`Serpiente`
      (`PrimitiveComponent.SetMaterial` (`self.CardImage`) 0 "/Game/WoN/Assets/Materials/Serpiente.Serpiente"))))

(event `CreateCreatureCard`
  (params (`Card Values Type` :type "/Game/WoN/Blueprints/Cards/Lists/CardTypes Enum" :default "NewEnumerator0"))
  ;[1 1 1] Crear carta criatura aleatoria
  (bind _output_get (set `self.CardValues` (make `/Game/WoN/Blueprints/Cards/card_structure` (`|GetEnumeratorNameAsString` (cast `/Game/WoN/Blueprints/Cards/Lists/CreatureNames` (`KismetMathLibrary.Conv_IntToByte` (`KismetMathLibrary.RandomIntegerInRange` 0 (- (enumcount `/Game/WoN/Blueprints/Cards/Lists/CreatureNames`) 1))))) `Card Values Type` false (`KismetMathLibrary.RandomIntegerInRange` 1 3) (`KismetMathLibrary.RandomIntegerInRange` 1 3) (make `/Game/WoN/Blueprints/Cards/card_skill` (`|GetEnumeratorNameAsString` (cast `/Game/WoN/Blueprints/Cards/Lists/SkillTypes` (`KismetMathLibrary.Conv_IntToByte` (`KismetMathLibrary.RandomIntegerInRange` 0 (- (enumcount `/Game/WoN/Blueprints/Cards/Lists/SkillTypes`) 1)))))))))
  (`self.SetCard` (break `/Game/WoN/Blueprints/Cards/card_structure` _output_get) (`.type_13_F085F1A24DDBC6A14069BAB5E01BBD77` (break `/Game/WoN/Blueprints/Cards/card_structure` _output_get)) (`.LP_14_8791EBD0490EC0BB729555B16F974E8B` (break `/Game/WoN/Blueprints/Cards/card_structure` _output_get)) (`.AP_15_6B4075BA4085D17E9D16BD811E139140` (break `/Game/WoN/Blueprints/Cards/card_structure` _output_get)) (break `/Game/WoN/Blueprints/Cards/card_skill` (`.skills_16_283604F149EFA84DAD296EBF29A55589` (break `/Game/WoN/Blueprints/Cards/card_structure` _output_get))))
  (bind _output_get_2 (set `self.numMana` (`KismetMathLibrary.RandomIntegerInRange` 1 2)))
  (`TextRenderComponent.K2_SetText` (`self.NeededMana`) (`KismetTextLibrary.Conv_IntToText` _output_get_2)))

(event `SetCardSkill`
  (params (`My Values Name` :type String) (`My Values Description` :type String) (`My Values Type` :type "/Game/WoN/Blueprints/Cards/Lists/SkillTypes Enum" :default "NewEnumerator0") (`Skill Necessary Mana` :type Integer))
  ;[1 1 1] Set card skill
  (set `self.Skill` (make `/Game/WoN/Blueprints/Cards/card_skill` `My Values Name` `My Values Description` `My Values Type`)))

(event `SetCardMaterial`
  (bind _material (`self.Material`))
  (bind (_cardvalues_name _cardvalues_type) (break `/Game/WoN/Blueprints/Cards/card_structure` (`self.CardValues`)))
  ;[1 1 1] Set Card Material (Different material due to Card Type)
  (switch `/Game/WoN/Blueprints/Cards/Lists/CardTypes` _cardvalues_type
    (:`NewEnumerator0`
      (set `self.Material` "/Game/Puzzle/Meshes/BaseMaterial.BaseMaterial"))
    (:`NewEnumerator1`
      (set `self.Material` "/Game/WoN/Assets/Materials/Land_Card.Land_Card"))
    (:`NewEnumerator2`
      (set `self.Material` "/Game/WoN/Assets/Materials/Spell_Card.Spell_Card"))
    (:`NewEnumerator3`
      (set `self.Material` "/Game/WoN/Assets/Materials/Criature_Card.Criature_Card"))
    (:`NewEnumerator4`
      (set `self.Material` "/Game/WoN/Assets/Materials/Object_Card.Object_Card")))
  (`PrimitiveComponent.SetMaterial` (`self.CardBody`) 0 _material)
  (`PrimitiveComponent.SetMaterial` (`self.cube`) 0 _material)
  (`PrimitiveComponent.SetMaterial` (`self.cube1`) 0 _material))

(event `SetLifeToZero`
  ;[1 1 1] Set life to zero
  (set `self.CardValues` (make `/Game/WoN/Blueprints/Cards/card_structure` "" "NewEnumerator3")))

(event `SetCard`
  (params (`Card Values Name` :type String) (`Card Values Type` :type "/Game/WoN/Blueprints/Cards/Lists/CardTypes Enum" :default "NewEnumerator0") (`Card Values LP` :type Integer) (`Card Values AP` :type Integer) (`Card Values Skills Name` :type String))
  (bind _cardvalues (`self.CardValues`))
  ;[1 1 1] Set card values
  (set `self.CardValues` (make `/Game/WoN/Blueprints/Cards/card_structure` `Card Values Name` `Card Values Type` false `Card Values LP` `Card Values AP` (make `/Game/WoN/Blueprints/Cards/card_skill` `Card Values Skills Name`)))
  (`TextRenderComponent.K2_SetText` (`self.CardName`) (`KismetTextLibrary.Conv_StringToText` (break `/Game/WoN/Blueprints/Cards/card_structure` _cardvalues)))
  (`TextRenderComponent.K2_SetText` (`self.CardDefenseTotal`) (`KismetTextLibrary.Conv_IntToText` (`.LP_14_8791EBD0490EC0BB729555B16F974E8B` (break `/Game/WoN/Blueprints/Cards/card_structure` _cardvalues))))
  (`TextRenderComponent.K2_SetText` (`self.CardDamage`) (`KismetTextLibrary.Conv_IntToText` (`.AP_15_6B4075BA4085D17E9D16BD811E139140` (break `/Game/WoN/Blueprints/Cards/card_structure` _cardvalues))))
  (`self.SetCardMaterial`)
  (`TextRenderComponent.K2_SetText` (`self.SkillText`) (`KismetTextLibrary.Conv_StringToText` (break `/Game/WoN/Blueprints/Cards/card_skill` (`.skills_16_283604F149EFA84DAD296EBF29A55589` (break `/Game/WoN/Blueprints/Cards/card_structure` _cardvalues)))))
  (`self.SetCreatureImage` (break `/Game/WoN/Blueprints/Cards/card_structure` _cardvalues)))

(event `ModValues`
  (params (ataque :type Integer) (vida :type Integer))
  (bind _cardvalues (`self.CardValues`))
  ;[1 1 1] Mod Values
  (`self.SetCard` (break `/Game/WoN/Blueprints/Cards/card_structure` _cardvalues) (`.type_13_F085F1A24DDBC6A14069BAB5E01BBD77` (break `/Game/WoN/Blueprints/Cards/card_structure` _cardvalues)) (+ vida (`.LP_14_8791EBD0490EC0BB729555B16F974E8B` (break `/Game/WoN/Blueprints/Cards/card_structure` _cardvalues))) (+ ataque (`.AP_15_6B4075BA4085D17E9D16BD811E139140` (break `/Game/WoN/Blueprints/Cards/card_structure` _cardvalues))) (break `/Game/WoN/Blueprints/Cards/card_skill` (`.skills_16_283604F149EFA84DAD296EBF29A55589` (break `/Game/WoN/Blueprints/Cards/card_structure` _cardvalues)))))

(event `self.ReceiveBeginPlay`
  (bind (_cardvalues_name _cardvalues_type _cardvalues_state _cardvalues_lp _cardvalues_ap) (break `/Game/WoN/Blueprints/Cards/card_structure` (`self.CardValues`)))
  (bind (_skill_name _skill_description _skill_type) (break `/Game/WoN/Blueprints/Cards/card_skill` (`self.Skill`)))
  ;[1 1 1] Inicializar valores carta (por defecto)
  (set `self.Skill` (make `/Game/WoN/Blueprints/Cards/card_skill` "" "" "NewEnumerator7"))
  (`self.SetCardSkill` _skill_name _skill_description _skill_type)
  (set `self.CardValues` (make `/Game/WoN/Blueprints/Cards/card_structure` "Tronchamulas" "NewEnumerator3" false 1 1))
  (`self.SetCard` _cardvalues_name _cardvalues_type _cardvalues_lp _cardvalues_ap)
  (bind _returnvalue (`|CreateWidget` "/Game/WoN/Blueprints/UI/CastCreature.CastCreature_C" null null))
  (set `self.CAST_UI` _returnvalue))

(event `SetCardLocation`
  (params (myNewPosition :type "Vector Structure"))
  ;[1 1 1] Set card location (for reposition use only)
  (`self.K2_SetActorLocation` myNewPosition))

(event `self.ReceiveActorOnClicked`
  (params (ButtonPressed :type "Key Structure"))
  ;[1 1 1] Click on Creature card
  (if (`self.isShown?`)
    (set `self.isShown?` false)
    (`self.K2_SetActorLocation` (`self.posInicial`))
    (`self.SetActorRelativeScale3D` (1.0 1.0 1.0))
    (`self.K2_SetActorRelativeRotation` (struct :`Yaw` 90.0 :`Roll` -90.0))
    (`TextRenderComponent.SetXScale` (`self.CardName`) 1.0)
    (`TextRenderComponent.SetXScale` (`self.NeededMana`) 1.0)
    (`TextRenderComponent.SetXScale` (`self.CardDamage`) 1.0)
    (`TextRenderComponent.SetXScale` (`self.CardDefenseTotal`) 1.0)
    (`TextRenderComponent.SetXScale` (`self.SkillText`) 1.0)
    (`Widget.RemoveFromParent` (`self.CAST_UI`))
    (else
      (set `self.isShown?` true)
      (`self.Mostrar Carta`))))

(event `Mostrar Carta`
  (bind _cast_ui (`self.CAST_UI`))
  ;[1 1 1] Mostrar carta "en grande"
  (`self.K2_SetActorLocation` (-90.0 -21.0 319.0))
  (`self.SetActorRelativeScale3D` (3.0 1.0 3.0))
  (`self.K2_SetActorRotation` (struct :`Yaw` 90.0 :`Roll` -68.400002))
  (`TextRenderComponent.SetXScale` (`self.CardName`) 4.5)
  (`TextRenderComponent.SetXScale` (`self.CardDamage`) 2.0)
  (`TextRenderComponent.SetXScale` (`self.CardDefenseTotal`) 2.0)
  (`TextRenderComponent.SetXScale` (`self.SkillText`) 3.0)
  (bind _outactors (`GameplayStatics.GetAllActorsOfClass` "/Game/WoN/Blueprints/Tablero/Tablero.Tablero_C"))
  (for _ _outactors
    (`TextRenderComponent.SetXScale` (`self.NeededMana`) 2.0)
    (set `/Game/WoN/Blueprints/UI/CastCreature.CreatureCard_CastUI` self _cast_ui)
    (if (not (`self.isCasted?`))
      (`UserWidget.AddToViewport` _cast_ui 0))))

(fn `UserConstructionScript`)