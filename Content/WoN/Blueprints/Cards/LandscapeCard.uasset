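; LandscapeCard is a clickable card actor for a landscape (Escenario) card in a card game.
; On BeginPlay it rolls a random land name and mana cost, then SetCard applies name text, body material by type and artwork by name.
; Clicking toggles an enlarged view at a fixed position, showing the CastLandscape widget if uncast and a Tablero exists.
; Creature artwork switching and a deprecated, unreachable debug-print chain are also present.
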(event `SetCreatureImage`
  (params (A :type String))
  ;[1 1 1] Set Creature Image
  (switch `string` A
    (:`Perro Salvaje`
      (`PrimitiveComponent.SetMaterial` (`self.CardImage`) 0 "/Game/WoN/Assets/Materials/Perro.Perro"))
    (:`Salaryman`
      (`PrimitiveComponent.SetMaterial` (`self.CardImage`) 0 "/Game/WoN/Assets/Materials/Salaryman.Salaryman"))
    (:`Abuelita`
      (`PrimitiveComponent.SetMaterial` (`self.CardImage`) 0 "/Game/WoN/Assets/Materials/Abuelita.Abuelita"))
    (:`Patata`
      (`PrimitiveComponent.SetMaterial` (`self.CardImage`) 0 "/Game/WoN/Assets/Materials/Patata.Patata"))
    (:`Tronchamulas`
      (`PrimitiveComponent.SetMaterial` (`self.CardImage`) 0 "/Game/WoN/Assets/Materials/Tronchamulas.Tronchamulas"))
    (:`Gato negro`
      (`PrimitiveComponent.SetMaterial` (`self.CardImage`) 0 "/Game/WoN/Assets/Materials/GatoNegro.GatoNegro"))
    (:`Asesino`
      (`PrimitiveComponent.SetMaterial` (`self.CardImage`) 0 "/Game/WoN/Assets/Materials/Asesino.Asesino"))
    (:`Barbol`
      (`PrimitiveComponent.SetMaterial` (`self.CardImage`) 0 "/Game/WoN/Assets/Materials/Barbol.Barbol"))
    (:`Filemon`
      (`PrimitiveComponent.SetMaterial` (`self.CardImage`) 0 "/Game/WoN/Assets/Materials/Filemon.Filemon"))
    (:`Tortuga`
      (`PrimitiveComponent.SetMaterial` (`self.CardImage`) 0 "/Game/WoN/Assets/Materials/Tortuga.Tortuga"))
    (:`Serpiente`
      (`PrimitiveComponent.SetMaterial` (`self.CardImage`) 0 "/Game/WoN/Assets/Materials/Serpiente.Serpiente"))))

(event `SetCardLocation`
  (params (myNewPosition :type "Vector Structure"))
  ;[1 1 1] Set card location (for reposition use only)
  (`self.K2_SetActorLocation` myNewPosition))

(event `CreateLandscapeCard`
  (params (PosInicial :type "Vector Structure"))
  ;[1 1 1] Create Landscape Card
  (bind _output_get (set `self.CardValues` (make `/Game/WoN/Blueprints/Cards/card_structure` (`|GetEnumeratorNameAsString` (cast `/Game/WoN/Blueprints/Cards/Lists/LandName` (`KismetMathLibrary.Conv_IntToByte` (`KismetMathLibrary.RandomIntegerInRange` 0 (- (enumcount `/Game/WoN/Blueprints/Cards/Lists/LandName`) 1))))) "NewEnumerator1")))
  (`self.SetCard` (break `/Game/WoN/Blueprints/Cards/card_structure` _output_get) "NewEnumerator1")
  (bind _output_get_2 (set `self.numMana` (`KismetMathLibrary.RandomIntegerInRange` 1 2)))
  (`TextRenderComponent.K2_SetText` (`self.NeededMana`) (`KismetTextLibrary.Conv_IntToText` _output_get_2))
  (set `self.posInicial` PosInicial))

(event `SetCardSkill`
  (params (`My Values Name` :type String) (`My Values Description` :type String) (`My Values Type` :type "/Game/WoN/Blueprints/Cards/Lists/SkillTypes Enum" :default "NewEnumerator0") (`Skill Necessary Mana` :type Integer))
  ;[1 1 1] Set card skill
  (set `self.Skill` (make `/Game/WoN/Blueprints/Cards/card_skill` `My Values Name` `My Values Description` `My Values Type`)))

(event `SetManaImage`
  (params (Image :type String))
  ;[1 1 1] Set Mana Image
  (switch `string` Image
    (:`Pradera`
      (`PrimitiveComponent.SetMaterial` (`self.CardImage`) 0 "/Game/WoN/Assets/Materials/Pradera.Pradera"))
    (:`Montaña`
      (`PrimitiveComponent.SetMaterial` (`self.CardImage`) 0 "/Game/WoN/Assets/Materials/Montaña.Montaña"))
    (:`Playa`
      (`PrimitiveComponent.SetMaterial` (`self.CardImage`) 0 "/Game/WoN/Assets/Materials/Playa.Playa"))
    (:`Ciudad`
      (`PrimitiveComponent.SetMaterial` (`self.CardImage`) 0 "/Game/WoN/Assets/Materials/Ciudad.Ciudad"))))

(event `SetCardMaterial`
  (bind (_cardvalues_name _cardvalues_type) (break `/Game/WoN/Blueprints/Cards/card_structure` (`self.CardValues`)))
  ;[1 1 1] Set Card Material (Different material due to Card Type)
  (switch `/Game/WoN/Blueprints/Cards/Lists/CardTypes` _cardvalues_type
    (:`NewEnumerator0`
      (set `self.Material` "/Game/Puzzle/Meshes/BaseMaterial.BaseMaterial"))
    (:`NewEnumerator1`
      (set `self.Material` "/Game/WoN/Assets/Materials/Land_Card.Land_Card"))
    (:`NewEnumerator2`
      (set `self.Material` "/Game/WoN/Assets/Materials/Spell_Card.Spell_Card"))
    (:`NewEnumerator3`
      (set `self.Material` "/Game/WoN/Assets/Materials/Criature_Card.Criature_Card"))
    (:`NewEnumerator4`
      (set `self.Material` "/Game/WoN/Assets/Materials/Object_Card.Object_Card")))
  (`PrimitiveComponent.SetMaterial` (`self.CardBody`) 0 (`self.Material`)))

(event `SetCard`
  (params (`Card Values Name` :type String) (`Card Values Type` :type "/Game/WoN/Blueprints/Cards/Lists/CardTypes Enum" :default "NewEnumerator0") (`Card Values LP` :type Integer) (`Card Values AP` :type Integer) (`Card Values Skills Name` :type String))
  (bind _cardvalues (`self.CardValues`))
  ;[1 1 1] Set card values
  (set `self.CardValues` (make `/Game/WoN/Blueprints/Cards/card_structure` `Card Values Name` `Card Values Type` false `Card Values LP` `Card Values AP` (make `/Game/WoN/Blueprints/Cards/card_skill` `Card Values Skills Name` "" "NewEnumerator7")))
  (`TextRenderComponent.K2_SetText` (`self.CardName`) (`KismetTextLibrary.Conv_StringToText` (break `/Game/WoN/Blueprints/Cards/card_structure` _cardvalues)))
  (`self.SetCardMaterial`)
  (`self.SetCreatureImage` (break `/Game/WoN/Blueprints/Cards/card_structure` _cardvalues))
  (`self.SetManaImage` (break `/Game/WoN/Blueprints/Cards/card_structure` _cardvalues)))

(event `self.ReceiveBeginPlay`
  ;[1 1 1] Inicializar valores carta (por defecto)
  (`self.CreateLandscapeCard` (0.0 0.0 0.0))
  (bind _returnvalue (`|CreateWidget` "/Game/WoN/Blueprints/UI/CastLandscape.CastLandscape_C" null null))
  (set `self.CAST_UI` _returnvalue))

(event `self.ReceiveActorOnClicked`
  (params (ButtonPressed :type "Key Structure"))
  ;[1 1 1] Click on Creature card
  (if (`self.isShown?`)
    (set `self.isShown?` false)
    (`self.K2_SetActorLocation` (`self.posInicial`))
    (`self.SetActorRelativeScale3D` (1.0 1.0 1.0))
    (`self.K2_SetActorRelativeRotation` (struct :`Yaw` 90.0 :`Roll` -90.0))
    (`TextRenderComponent.SetXScale` (`self.CardName`) 1.0)
    (`TextRenderComponent.SetXScale` (`self.NeededMana`) 1.0)
    (`Widget.RemoveFromParent` (`self.CAST_UI`))
    (else
      (set `self.isShown?` true)
      (`self.Mostrar Carta`))))

(event `Mostrar Carta`
  (bind _cast_ui (`self.CAST_UI`))
  ;[1 1 1] Mostrar carta "en grande"
  (`self.K2_SetActorLocation` (-90.0 -21.0 319.0))
  (`self.SetActorRelativeScale3D` (3.0 1.0 3.0))
  (`self.K2_SetActorRotation` (struct :`Yaw` 90.0 :`Roll` -68.400002))
  (`TextRenderComponent.SetXScale` (`self.CardName`) 4.5)
  (bind _outactors (`GameplayStatics.GetAllActorsOfClass` "/Game/WoN/Blueprints/Tablero/Tablero.Tablero_C"))
  (for _ _outactors
    (`TextRenderComponent.SetXScale` (`self.NeededMana`) 2.0)
    (set `/Game/WoN/Blueprints/UI/CastLandscape.LandscapeCard_CastUI` self _cast_ui)
    (if (not (`self.isCasted?`))
      (`UserWidget.AddToViewport` _cast_ui 0))))

(fn `UserConstructionScript`)